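; Base enemy character that hunts and melees the IA主角 player, with a health-bar widget.
; PawnSensing writes the seen player to the Blackboard as the attack target.
; Random attack montages sphere-trace forward on notify to deal damage, then fire an attack-finished dispatcher.
; Hits reduce health and play a movement-locking reaction through server-to-multicast events; death removes the bar and, given a valid killer, credits the kill, disables collision and destroys the actor after a delay.
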(event OnSeePawn(PawnSensing)
  (params (Pawn :type Pawn%20Object%20Reference))
  ;[0.15 0.15 0.15 0.5] 感知主角
  (bind _asia主角 (Utilities|Casting|CastToIA主角 Pawn))
  (AI|Components|Blackboard|SetValueasObject (AI|GetBlackboard 0) (Utilities|Name|MakeLiteralName "攻击目标") _asia主角))

(event Custom|受到攻击
  (params (伤害值 :type Float%20%28double-precision%29) (谁打的 :type IA主角%20Object%20Reference))
  ;[0.15 0.15 0.15 0.5] 受到攻击掉血或死亡
  (Variables|Default|Set谁打的 谁打的)
  (if (> (Variables|Default|Get当前生命) 0.0)
    (bind _output_get (Variables|Default|Set当前生命 (- (Variables|Default|Get当前生命) 伤害值)))
    (if (<= _output_get 0.0)
      (Variables|Default|Set死亡否 true)
      (Components|DestroyComponent (Variables|Default|GetWidget1))
      (bind _谁打的 (Variables|Default|Get谁打的)
        (:then
          (Variables|/Game/自设蓝图/IA主角.IA主角_C|Set击杀数 _谁打的 (+ (Variables|/Game/自设蓝图/IA主角.IA主角_C|Get击杀数 _谁打的) 1))
          (Collision|SetCollisionEnabled (Variables|Collision|GetCapsuleComponent) "NoCollision")
          (Collision|SetCollisionEnabled (Variables|Character|GetMesh) "NoCollision")
          (Utilities|FlowControl|Delay 3.0)
          (Actor|DestroyActor))
        (:else))
      (else
        (CallFunction|服务器 (Variables|Default|Get受击蒙太奇))))))

(event Custom|组播
  (params (MontageToPlay :type Anim%20Montage%20Object%20Reference))
  ;[0.15 0.15 0.15 0.5] 受到攻击掉血或死亡
  (Animation|Montage|PlayMontage (Variables|Character|GetMesh) MontageToPlay
    (:then
      (Pawn|Components|CharacterMovement|SetMovementMode (Variables|Character|GetCharacterMovement) "MOVE_None" 0)
      (Variables|/Script/Engine.CharacterMovementComponent|SetMaxWalkSpeed (Variables|Character|GetCharacterMovement) 0.0))
    (:OnCompleted
      (Pawn|Components|CharacterMovement|SetMovementMode (Variables|Character|GetCharacterMovement) "MOVE_Walking" 0)
      (Variables|/Script/Engine.CharacterMovementComponent|SetMaxWalkSpeed (Variables|Character|GetCharacterMovement) 375.0))))

(event Custom|服务器
  (params (MontageToPlay :type Anim%20Montage%20Object%20Reference))
  ;[0.15 0.15 0.15 0.5] 受到攻击掉血或死亡
  (CallFunction|组播 MontageToPlay))

(event Custom|敌人播放攻击
  ;[0.15 0.15 0.15 0.5] 攻击IA主角
  (CallFunction|敌人组播攻击 (.OutItem (Utilities|Array|Random (Variables|Default|Get攻击蒙太奇组)))))

(event Custom|敌人组播攻击
  (params (MontageToPlay :type Anim%20Montage%20Object%20Reference))
  (bind _returnvalue (Transformation|GetActorLocation))
  ;[0.15 0.15 0.15 0.5] 攻击IA主角
  (bind _notifyname (Animation|Montage|PlayMontage (Variables|Character|GetMesh) MontageToPlay)
    (:OnCompleted
      _)
    (:OnInterrupted
      _)
    (:OnNotifyBegin
      (switch name _notifyname
        (:敌人攻击伤害
          (bind _outhits (Collision|MultiSphereTraceForObjects _returnvalue (+ _returnvalue (* (Transformation|GetActorForwardVector) 2e+02)) 5e+01 (Utilities|Array|MakeArray "ObjectTypeQuery3") false 0 "None"))
          (bind _array_element (Utilities|Array|ForEachLoopwithBreak _outhits :!label _label)
            (:LoopBody
              (bind _asia主角 (Utilities|Casting|CastToIA主角 (.HitActor (Collision|BreakHitResult _array_element))))
              (Default|受到攻击 _asia主角 (Math|Random|RandomFloatinRange 2e+01 3e+01))
              (goto _label Break)))))))
  (Default|Call攻击完成事件分发器))

(event EventBeginPlay
  ;[0.15 0.15 0.15 0.5] 初始设置血条
  (Variables|Default|Set生命上限 (Variables|Default|Get当前生命))
  (bind _returnvalue (UserInterface|CreateWidget "/Game/界面UI/敌人血条.敌人血条_C" 0 self))
  (UserInterface|SetWidget (Variables|Default|GetWidget1) _returnvalue))

(fn ConstructionScript)